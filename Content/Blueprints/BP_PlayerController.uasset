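; Player controller for a horror game that handles the player's death sequence.
; On death it unpossesses the pawn, fades the camera out and holds it, and shows the YouDied widget.
; After a short delay it removes the widget and calls RestartGame on BP_MyHorrorGameGameModeBase_LS.
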(event Custom|OnDeath
  (Pawn|UnPossess)
  (CameraFades|StartCameraFade :self (Variables|Default|GetPlayerCameraManager) :FromAlpha 0.0 :ToAlpha 1.0 :Duration 1.0 :bHoldWhenFinished true)
  (bind _returnvalue (UserInterface|CreateWidget "/Game/Blueprints/YouDied.YouDied_C" self))
  (UserInterface|Viewport|AddtoViewport _returnvalue 0)
  (Utilities|FlowControl|Delay 2.0)
  (Widget|RemovefromParent _returnvalue)
  (bind _asbp_my_horror_game_game_mode_base_ls (Utilities|Casting|CastToBP_MyHorrorGameGameModeBase_LS (Game|GetGameMode)))
  (Class|GameMode|RestartGame _asbp_my_horror_game_game_mode_base_ls))

(event EventBeginPlay)

(event EventTick
  (params (DeltaSeconds :type Float%20%28single-precision%29)))

(fn ConstructionScript)